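; Bow actor that lays out its string between upper and lower attachment points on the bow.
; The Construction Script finds their midpoint by stepping half their distance along a look-at direction.
; It then stretches the UpperString and LowerString spline meshes from their respective ends to meet at that point.
; The event graph holds only disabled default events, so there is no draw or firing logic.
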(event EventBeginPlay)

(event Collision|EventActorBeginOverlap
  (params (OtherActor :type Actor%20Object%20Reference)))

(event EventTick
  (params (DeltaSeconds :type Float%20%28single-precision%29)))

(fn ConstructionScript
  (bind _upperbowposition (Variables|Default|GetUpperbowposition))
  (bind _lowerbowposition (Variables|Default|GetLowerbowposition))
  (bind _relativelocation (Variables|/Script/Engine.SceneComponent|GetRelativeLocation _upperbowposition))
  (bind _relativelocation_2 (Variables|/Script/Engine.SceneComponent|GetRelativeLocation _lowerbowposition))
  (bind _output_get (Variables|Default|SetMidPoint (+ _relativelocation (* (/ (Math|Vector|Distance(Vector) _relativelocation _relativelocation_2) 2.0) (Math|Vector|GetForwardVector (Math|Rotator|FindLookatRotation _relativelocation _relativelocation_2))))))
  (SplineMesh|SetStartandEnd (Variables|Default|GetUpperString) (Variables|/Script/Engine.SceneComponent|GetRelativeLocation (Variables|Default|GetUpperbowposition)) "0, 0, 0" _output_get "0, 0, 0" true :!class /Script/Engine.SplineMeshComponent)
  (SplineMesh|SetStartandEnd (Variables|Default|GetLowerString) (Variables|/Script/Engine.SceneComponent|GetRelativeLocation (Variables|Default|GetLowerbowposition)) "0, 0, 0" _output_get "0, 0, 0" true :!class /Script/Engine.SplineMeshComponent))