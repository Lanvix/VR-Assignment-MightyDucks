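; VR two-handed bow Actor that attaches to the first grabbing motion controller and spawns an arrow on a second controller's grab.
; While a secondary controller is valid, Tick aims bow and arrow along the line between hands and stretches two spline-mesh string halves from a construction-computed midpoint.
; Release scales launch power by hand distance; a DoOnce in Tick then resets the string and fires.
; As written, Grab sets the secondary controller to None.
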(event EventTick
  (params (DeltaSeconds :type Float%20%28single-precision%29))
  (bind _primarymotioncontroller (Variables|Default|GetPrimaryMotionController))
  (bind _midpoint (Variables|Default|GetMidPoint))
  (bind _secondarymotioncontroller (Variables|Default|GetSecondaryMotionController)
    (:then
      (Transformation|SetActorRotation (Math|Rotator|MakeRotator (.roll (Transformation|GetWorldRotation _primarymotioncontroller)) (.pitch (Math|Rotator|FindLookatRotation (Transformation|GetWorldLocation _secondarymotioncontroller) (Transformation|GetWorldLocation _primarymotioncontroller))) (.yaw (Math|Rotator|FindLookatRotation (Transformation|GetWorldLocation _secondarymotioncontroller) (Transformation|GetWorldLocation _primarymotioncontroller)))))
      (SplineMesh|SetEndPosition (Variables|Default|GetUpperstring) (Math|Vector|MakeVector (/ (Math|Vector|Distance(Vector) (Transformation|GetWorldLocation (Variables|Default|GetPrimaryMotionController)) (Transformation|GetWorldLocation (Variables|Default|GetSecondaryMotionController))) (.x (Transformation|GetActorScale3D))) (.y _midpoint) (.z _midpoint)) true)
      (bind _arrow (Variables|Default|GetArrow)
        (:then
          (Transformation|SetActorLocationAndRotation _arrow (Transformation|GetWorldLocation (Variables|Default|GetSecondaryMotionController)) (Math|Rotator|MakeRotator (.roll (Transformation|GetWorldRotation _primarymotioncontroller)) (.pitch (Math|Rotator|FindLookatRotation (Transformation|GetWorldLocation _secondarymotioncontroller) (Transformation|GetWorldLocation _primarymotioncontroller))) (.yaw (Math|Rotator|FindLookatRotation (Transformation|GetWorldLocation _secondarymotioncontroller) (Transformation|GetWorldLocation _primarymotioncontroller)))))
          (goto _label Reset))
        (:else
          (goto _label Reset))))
    (:else
      (Utilities|FlowControl|DoOnce true :!label _label
        (:Completed
          (SplineMesh|SetEndPosition (Variables|Default|GetLowerstring) (Variables|Default|GetMidPoint) true)
          (Transformation|SetActorRelativeRotation "-90.000000, 0, 0")
          (bind _arrow_2 (Variables|Default|GetArrow)
            (:then
              (Default|Fire _arrow_2 (Variables|Default|GetMultiplier))
              (Variables|Default|SetArrow 0))
            (:else)))))))

(event EventRelease
  (params (MotionController :type Motion%20Controller%20Component%20Object%20Reference))
  (if (== MotionController (Variables|Default|GetSecondaryMotionController))
    (Variables|Default|SetMultiplier (* (Math|Vector|Distance(Vector) (Transformation|GetWorldLocation (Variables|Default|GetPrimaryMotionController)) (Transformation|GetWorldLocation (Variables|Default|GetSecondaryMotionController))) 1e+04))
    (Variables|Default|SetSecondaryMotionController 0)
    (else
      (Variables|Default|SetPrimaryMotionController 0)
      (Variables|Default|SetSecondaryMotionController 0)
      (Transformation|DetachFromActor "KeepWorld" "KeepWorld" "KeepWorld"))))

(event EventGrab
  (params (MotionController :type Motion%20Controller%20Component%20Object%20Reference))
  (bind _primarymotioncontroller (Variables|Default|GetPrimaryMotionController)
    (:then
      (if (!= _primarymotioncontroller MotionController)
        (Variables|Default|SetSecondaryMotionController 0)
        (bind _returnvalue (Game|SpawnActorfromClass "/Game/Blueprints/Arrow.Arrow_C" (Math|Transform|MakeTransform "0, 0, 0" "0, 0, 0" "1.000000,1.000000,1.000000") "AlwaysSpawn" 0 0))
        (Variables|Default|SetArrow _returnvalue)))
    (:else
      (bind _output_get (Variables|Default|SetPrimaryMotionController MotionController))
      (Transformation|AttachComponentToComponent _output_get "None" "SnapToTarget" "SnapToTarget" "KeepWorld" true)
      (Transformation|SetActorRelativeRotation "-90.000000, 0, 0"))))

(fn ConstructionScript
  (bind _upperbowposition (Variables|Default|GetUpperbowposition))
  (bind _lowerbowposition (Variables|Default|GetLowerbowposition))
  (bind _relativelocation (Variables|/Script/Engine.SceneComponent|GetRelativeLocation _upperbowposition))
  (bind _relativelocation_2 (Variables|/Script/Engine.SceneComponent|GetRelativeLocation _lowerbowposition))
  (bind _output_get (Variables|Default|SetMidPoint (+ _relativelocation (* (/ (Math|Vector|Distance(Vector) _relativelocation _relativelocation_2) 2.0) (Math|Vector|GetForwardVector (Math|Rotator|FindLookatRotation _relativelocation _relativelocation_2))))))
  (SplineMesh|SetStartandEnd (Variables|Default|GetUpperstring) (Variables|/Script/Engine.SceneComponent|GetRelativeLocation (Variables|Default|GetUpperbowposition)) "0, 0, 0" _output_get "0, 0, 0" true :!class /Script/Engine.SplineMeshComponent)
  (SplineMesh|SetStartandEnd (Variables|Default|GetLowerstring) (Variables|/Script/Engine.SceneComponent|GetRelativeLocation (Variables|Default|GetLowerbowposition)) "0, 0, 0" _output_get "0, 0, 0" true :!class /Script/Engine.SplineMeshComponent))